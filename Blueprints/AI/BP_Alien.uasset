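; Spider-like alien enemy that chases the player with a looping AI MoveTo, re-issued shortly after each success or failure.
; Each tick, when close to the marine, it halts movement and plays an attack montage.
; A marine overlapping component S damages the alien itself, not the marine.
; Damage updates its health widget; at zero health it spawns an emitter, plays a death animation and is destroyed after a delay.
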(event `self.ReceiveBeginPlay`
  (`|AIMoveTo` self (0.0 0.0 0.0) (`GameplayStatics.GetPlayerCharacter` 0) :!label _label
    (:`then`
      (bind _asw_alienek (cast `/Game/UI/W_Alienek` (`WidgetComponent.GetUserWidgetObject` (`self.Widget`))))
      (bind _output_get (set `self.As W Alienek` _asw_alienek))
      (set `/Game/UI/W_Alienek.Curr_health` (`self.current healt`) _output_get)
      (set `/Game/UI/W_Alienek.Max_health` (`self.max healt`) _output_get))
    (:`OnSuccess`
      (`KismetSystemLibrary.Delay` 0.2 :!label _label_2)
      (goto _label))
    (:`OnFail`
      (goto _label_2))))

(event `self.ReceiveTick`
  (params (DeltaSeconds :type "Float (single-precision)"))
  ;[1 1 1] spider attack
  (if (`self.Is_atack_range`)
    (if (not (`self.is_atacking_?`))
      (`ActorComponent.Deactivate` (`self.CharacterMovement`))
      (`|PlayMontage` (`self.Mesh`) "/Game/Characters/Enemy_Great_Spider/Animations/Animation_montage_spider_atack.Animation_montage_spider_atack"
        (:`OnCompleted`
          (`ActorComponent.Activate` (`self.CharacterMovement`) false))))))

(event `self.s.OnComponentBeginOverlap`
  (params (OverlappedComponent :type "PrimitiveComponent Object Reference") (OtherActor :type "Actor Object Reference") (OtherComp :type "PrimitiveComponent Object Reference") (OtherBodyIndex :type Integer) (bFromSweep :type Boolean) (SweepResult :type "HitResult Structure (by ref)"))
  (cast `/Game/Blueprints/Pawns/BP_Marine` OtherActor)
  (`GameplayStatics.ApplyDamage` self 0.5))

(event `self.ReceiveAnyDamage`
  (params (Damage :type "Float (single-precision)") (DamageType :type "DamageType Object Reference") (InstigatedBy :type "Controller Object Reference") (DamageCauser :type "Actor Object Reference"))
  (bind _output_get (set `self.current healt` (- (`self.current healt`) (`KismetMathLibrary.FTrunc` (* Damage 100.0)))))
  (`/Game/UI/W_Alienek.update health` (`self.As W Alienek`) (`KismetMathLibrary.Clamp` _output_get 0 (`self.max healt`)))
  (if (<= (`self.current healt`) 0)
    (`GameplayStatics.SpawnEmitterAttached` null (`self.CapsuleComponent`))
    (`SkeletalMeshComponent.PlayAnimation` (`self.Mesh`) "/Game/Characters/Marine/Animations/Death.Death" false)
    (`KismetSystemLibrary.Delay` 2.0)
    (`self.K2_DestroyActor`)))

(fn `Is_atack_range`
  (returns (ReturnValue :type Boolean))
  (bind _asbp_marine (cast `/Game/Blueprints/Pawns/BP_Marine` (`GameplayStatics.GetPlayerPawn` 0)))
  (return (< (`self.GetDistanceTo` _asbp_marine) 100.0)))

(fn `is_atacking_?`
  (returns (ReturnValue :type Boolean))
  (return (`AnimInstance.Montage_IsPlaying` (`SkeletalMeshComponent.GetAnimInstance` (`self.Mesh`)) null)))

(fn `UserConstructionScript`)